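; Brick cube variant for an Arcanoid game that can drop a bonus when destroyed.
; On BeginPlay it checks whether the cube's first material is M_Sharic and only then binds a spawn handler to its OnDestroyed event.
; The handler always spawns BP_Bonus at the cube's location with a fixed rotation.
; Hit handling and construction simply call the parent implementations.
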(event `self.ReceiveBeginPlay`
  (if (== (`PrimitiveComponent.GetMaterial` (`self.Cube`) 0) "/Game/Arcanoid/Materials/Matals/M_Sharic.M_Sharic")
    ;[1 1 1] Spawn Bonus
    (add `self.OnDestroyed` (delegate `SpawnBonus`))))

(event `SpawnBonus` :!signature `self.OnDestroyed`
  (params (DestroyedActor :type "Actor Object Reference"))
  ;[1 1 1] Spawn Bonus
  (`|SpawnActorFromClass` "/Game/Arcanoid/Blueprints/Bonus/BP_Bonus.BP_Bonus_C" (`KismetMathLibrary.MakeTransform` (`self.K2_GetActorLocation`) (struct :`Pitch` -90.0 :`Yaw` -5.0)) "AlwaysSpawn" "OverrideRootScale" null null))

(event `self.BullHit`
  (`parent.BullHit`))

(fn `UserConstructionScript`
  (`parent.UserConstructionScript`))