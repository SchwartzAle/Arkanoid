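; Player controller for an Arcanoid-style game that sets game-only input and shows the WBP_Livel HUD widget on BeginPlay.
; On possess it caches the pawn as BP_Pawn.
; The MoveRight axis slides that pawn along world Y with a swept, frame-rate-independent offset scaled by Speed.
; The SpawnBoll action calls the pawn's SpawnShrick function.
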(event `self.ReceiveBeginPlay`
  (`WidgetBlueprintLibrary.SetInputMode_GameOnly` self)
  (bind _returnvalue (`|CreateWidget` "/Game/Arcanoid/UI/WBP_Livel.WBP_Livel_C" self))
  (`UserWidget.AddToViewport` _returnvalue 0)
  (set `self.Hud` _returnvalue))

(event `self.ReceivePossess`
  (params (PossessedPawn :type "Pawn Object Reference"))
  (bind _asbp_pawn (cast `/Game/Arcanoid/Blueprints/COre/BP_Pawn` PossessedPawn))
  (set `self.MyPawn` _asbp_pawn))

(event `InputAxis|MoveRight`
  (params (AxisValue :type "Float (single-precision)"))
  (`self.K2_AddActorWorldOffset` (`self.MyPawn`) (`KismetMathLibrary.MakeVector` 0.0 (* AxisValue (`GameplayStatics.GetWorldDeltaSeconds`) (`self.Speed`))) true false))

(event `InputAction|SpawnBoll`
  (params (Key :type "Key Structure"))
  (:`Pressed`
    (`/Game/Arcanoid/Blueprints/COre/BP_Pawn.SpawnShrick` (`self.MyPawn`))))

(fn `UserConstructionScript`)