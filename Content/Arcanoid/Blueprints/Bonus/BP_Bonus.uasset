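; BP_Bonus is a bonus pickup actor for the Arcanoid game that moves across the level.
; The construction script randomly picks one of three bonus types (MAX, Live or Ball) and gives the Cube component a matching mesh.
; Tick moves the actor in X and Y along Direction at Speed, scaled by delta time and with sweep enabled.
; The file holds no overlap or pickup logic.
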(event `self.ReceiveTick`
  (params (DeltaSeconds :type "Float (single-precision)"))
  (bind (_returnvalue_x _returnvalue_y) (`KismetMathLibrary.BreakVector` (* (`self.Direction`) (* DeltaSeconds (`self.Speed`)))))
  ;[1 1 1] Dvijenie bonusa
  (`self.K2_AddActorWorldOffset` (`KismetMathLibrary.MakeVector` _returnvalue_x _returnvalue_y) true))

(fn `UserConstructionScript`
  (bind _cube (`self.Cube`))
  ;[1 1 1] Rundom Bonus
  ;[1 1 1] figuri dlya bonus
  (bind _output_get (set `self.Bonus` (select `int` (`KismetMathLibrary.RandomIntegerInRange` 0 2) :`0` "NewEnumerator0" :`1` "NewEnumerator1" :`2` "NewEnumerator2" :!type "/Game/Arcanoid/Blueprints/Bonus/BonusType Enum")))
  (switch `/Game/Arcanoid/Blueprints/Bonus/BonusType` _output_get
    (:`NewEnumerator0`
      (`StaticMeshComponent.SetStaticMesh` _cube "/Game/Arcanoid/Materials/Matals/Serdce/christmas.christmas"))
    (:`NewEnumerator1`
      (`StaticMeshComponent.SetStaticMesh` _cube "/Game/Arcanoid/Materials/Matals/PUMPING_HEART_MODEL.PUMPING_HEART_MODEL"))
    (:`NewEnumerator2`
      (`StaticMeshComponent.SetStaticMesh` _cube "/Game/avtopapki/StarterContent/Props/MaterialSphere.MaterialSphere"))))