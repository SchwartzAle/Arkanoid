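; BP_CubeGenirator is a spawner that lays out the grid of cubes for an Arkanoid-style level.
; The construction script builds a static mesh preview from X, Y and the Rastoyaniye spacing.
; BeginPlay destroys the preview, then spawns BP_Cube_Child actors at matching offsets from its location and stores them in Cubes.
; GetCubesWin returns the cube count, but the win-count and death-binding logic is disconnected, and DeadCube is empty.
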(event `self.ReceiveBeginPlay`
  (bind (_returnvalue_x _returnvalue_y _returnvalue_z) (`KismetMathLibrary.BreakVector` (`self.K2_GetActorLocation`)))
  (for _array_element (`self.Prew`)
    (`ActorComponent.K2_DestroyComponent` _array_element))
  (for _index (range (+ (`self.X`) 1))
    (for _index_2 (range (+ (`self.Y`) 1))
      (bind _returnvalue (`|SpawnActorFromClass` "/Game/Arcanoid/Blueprints/BP_Cube_Child.BP_Cube_Child_C" (`KismetMathLibrary.MakeTransform` (`KismetMathLibrary.MakeVector` (+ _returnvalue_x (`KismetMathLibrary.Conv_IntToDouble` (* _index (`self.Rastoyaniye`)))) (+ _returnvalue_y (`KismetMathLibrary.Conv_IntToDouble` (* _index_2 (`self.Rastoyaniye`)))) _returnvalue_z)) "Undefined" "OverrideRootScale" null null))
      (`KismetArrayLibrary.Array_Add` (`self.Cubes`) _returnvalue))))

(event `DeadCube`
  (params (Score :type Integer)))

(fn `GetCubesWin`
  (returns (AmountCubs :type Integer))
  (return (`KismetArrayLibrary.Array_Length` (`self.Cubes`))))

(fn `UserConstructionScript`
  (for _index (range (+ (`self.X`) 1))
    (for _index_2 (range (+ (`self.Y`) 1))
      (bind _returnvalue (`AddComponent|NODE_AddStaticMeshComponent-0` :`RelativeTransform` (`KismetMathLibrary.MakeTransform` (`KismetMathLibrary.MakeVector` (`KismetMathLibrary.Conv_IntToDouble` (* _index (`self.Rastoyaniye`))) (`KismetMathLibrary.Conv_IntToDouble` (* _index_2 (`self.Rastoyaniye`)))))))
      (`KismetArrayLibrary.Array_Add` (`self.Prew`) _returnvalue))))