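; BP_Cube_Parent is the parent brick Blueprint for an Arkanoid-style game, destroyed by hits from the BP_Sharik ball.
; The construction script randomly gives each brick one or two lives (Jizn), with a matching material and Score value.
; A ball hit calls BullHit, which decrements Jizn, swapping the material at one life and destroying the actor at zero.
; The CallCubeDead dispatcher call is unconnected, so destruction never broadcasts it.
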(event `self.ReceiveBeginPlay`)

(event `self.ReceiveHit`
  (params (MyComp :type "PrimitiveComponent Object Reference") (Other :type "Actor Object Reference") (OtherComp :type "PrimitiveComponent Object Reference") (bSelfMoved :type Boolean) (HitLocation :type "Vector Structure") (HitNormal :type "Vector Structure") (NormalImpulse :type "Vector Structure") (Hit :type "HitResult Structure (by ref)"))
  (cast `/Game/Arcanoid/Blueprints/BP_Sharik` Other)
  (`self.BullHit`))

(event `BullHit`
  (bind _result (`/Engine/EditorBlueprintResources/StandardMacros.DecrementInt` (`self.Jizn`))
    (:`  `
      (if (== _result 1)
        (`PrimitiveComponent.SetMaterial` (`self.Cube`) 0 "/Game/Arcanoid/Materials/Matals/M_Sharic2.M_Sharic2")
        (elif (<= _result 0)
          (`self.K2_DestroyActor`))))))

(fn `UserConstructionScript`
  (bind _output_get (set `self.Jizn` (`KismetMathLibrary.RandomIntegerInRange` 1 2)))
  (switch `int` _output_get
    (:`1`
      (`PrimitiveComponent.SetMaterial` (`self.Cube`) 0 "/Game/Arcanoid/Materials/Matals/M_Sharic2.M_Sharic2")
      (set `self.Score` 50))
    (:`2`
      (`PrimitiveComponent.SetMaterial` (`self.Cube`) 0 "/Game/Arcanoid/Materials/Matals/M_Sharic.M_Sharic")
      (set `self.Score` 100))))